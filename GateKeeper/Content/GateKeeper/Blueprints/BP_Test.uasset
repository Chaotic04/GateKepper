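; BP_Test is a test actor with a spinning cylinder that damages what touches its capsule.
; Tick adds a Rotation variable to the cylinder's relative yaw each frame, without delta-time scaling.
; Capsule overlaps with components of one custom collision object type apply fixed damage to the owning actor.
; A Playerattackhit event only prints a debug string, and unconnected leftover nodes remain in the graph.
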(event OnComponentBeginOverlap(Capsule)
  (params (OverlappedComponent :type Primitive%20Component%20Object%20Reference) (OtherActor :type Actor%20Object%20Reference) (OtherComp :type Primitive%20Component%20Object%20Reference) (OtherBodyIndex :type Integer) (bFromSweep :type Boolean) (SweepResult :type Hit%20Result%20Structure%20%28by%20ref%29))
  (if (Utilities|Enum|Equal(Enum) (Collision|GetCollisionObjectType OtherComp) "ECC_GameTraceChannel2")
    (Utilities|IsValid OtherActor
      (:Is%20Valid
        (Game|Damage|ApplyDamage OtherActor 1e+01 0 0)))))

(event EventBeginPlay)

(event Collision|EventActorBeginOverlap
  (params (OtherActor :type Actor%20Object%20Reference)))

(event EventTick
  (params (DeltaSeconds :type Float%20%28single-precision%29))
  (bind _cylinder1 (Variables|Default|GetCylinder1))
  (Transformation|SetRelativeRotation _cylinder1 (Math|Rotator|MakeRotator 0.0 0.0 (+ (.yaw (Variables|/Script/Engine.SceneComponent|GetRelativeRotation _cylinder1)) (Variables|Default|GetRotation))) false false))

(event EventPlayerattackhit
  (Development|PrintString "ouchie"))

(fn ConstructionScript)